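; BP_Stage_Elevator is a stage Blueprint in an event test map that drives an elevator entity from stage state.
; State changes on the elevator's entity ID resolve its actor and send it to reset, top or bottom.
; Pressing E while act 1 is active alternates between activating acts 2 and 3.
; Load and activate zone handlers mostly print debug text, though leaving the activate zone calls LoadStage.
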(event OnActorEnter(BuiltInLoadZone)
  (params (Zone :type Trigger%20Zone%20Component%20Base%20Object%20Reference) (Actor :type Actor%20Object%20Reference))
  (Development|PrintString "load stage"))

(event OnActorExit(BuiltInLoadZone)
  (params (Zone :type Trigger%20Zone%20Component%20Base%20Object%20Reference) (Actor :type Actor%20Object%20Reference))
  (Development|PrintString "unload stage"))

(event OnActorEnter(BuiltInActivateZone)
  (params (Zone :type Trigger%20Zone%20Component%20Base%20Object%20Reference) (Actor :type Actor%20Object%20Reference))
  (Development|PrintString "activate stage"))

(event OnActorExit(BuiltInActivateZone)
  (params (Zone :type Trigger%20Zone%20Component%20Base%20Object%20Reference) (Actor :type Actor%20Object%20Reference))
  (Class|Stage|LoadStage))

(event EventBeginPlay
  (|CallParentFunction)
  (Input|EnableInput (Game|GetPlayerController 0)))

(event EventOnStageEntityStateChanged
  (params (EntityID :type Integer) (OldState :type Integer) (NewState :type Integer))
  (bind _elevator_entityid (Variables|Default|GetElevator%20EntityID))
  (if (== EntityID _elevator_entityid)
    (Variables|Default|SetElevator%20Ref (.AsBP%20Entity%20Actor%20Elevator (Utilities|Casting|CastToBP_EntityActor_Elevator (Class|Stage|GetEntityActorbyID _elevator_entityid))))
    (if (Utilities|IsValid (Variables|Default|GetElevator%20Ref))
      (switch int NewState
        (:0
          (Default|ResetLocation (Variables|Default|GetElevator%20Ref)))
        (:1
          (Default|GotoTop (Variables|Default|GetElevator%20Ref)))
        (:2
          (Default|GotoBottom (Variables|Default|GetElevator%20Ref))))
      (else
        (Development|PrintString "Entity Ref not Valid")))))

(event Input|KeyboardEvents|E
  (params (Key :type Key%20Structure :default "None"))
  (:Pressed
    (Development|PrintString "PreesE")
    (if (Class|Stage|IsActActive 1)
      (Utilities|FlowControl|FlipFlop
        (:A
          (Class|Stage|ActivateAct 2))
        (:B
          (Class|Stage|ActivateAct 3))))))

(fn ConstructionScript
  (|CallParentFunction))