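; Elevator entity actor that rises 500 units while something overlaps its foot collision and travels back down when the overlap ends.
; Overlap events set the EntityComponent state, whose change event plays the timeline from start, reverses it, or snaps to bottom.
; The timeline lerps between bottom and top locations, captured shortly after BeginPlay.
; Debug spheres and prints trace movement, state changes and owner stage ID.
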(event OnEntityStateChanged(EntityComponent)
  (params (NewState :type Integer) (OldState :type Integer))
  (bind _entitycomponent (Variables|Default|GetEntityComponent))
  (bind _returnvalue (Class|StageEntityComponent|GetOwnerStageID _entitycomponent))
  (bind _returnvalue_2 (Utilities|String|ToString(Integer) _returnvalue))
  (switch int NewState
    (:0
      (CallFunction|ResetLocation))
    (:1
      (Development|PrintString _returnvalue_2)
      (CallFunction|GotoTop))
    (:2
      (Development|PrintString _returnvalue_2)
      (CallFunction|GotoBottom))))

(event OnComponentBeginOverlap(FootCollision)
  (params (OverlappedComponent :type Primitive%20Component%20Object%20Reference) (OtherActor :type Actor%20Object%20Reference) (OtherComp :type Primitive%20Component%20Object%20Reference) (OtherBodyIndex :type Integer) (bFromSweep :type Boolean) (SweepResult :type Hit%20Result%20Structure%20%28by%20ref%29))
  (Class|StageEntityComponent|SetEntityState (Variables|Default|GetEntityComponent) 1 false))

(event OnComponentEndOverlap(FootCollision)
  (params (OverlappedComponent :type Primitive%20Component%20Object%20Reference) (OtherActor :type Actor%20Object%20Reference) (OtherComp :type Primitive%20Component%20Object%20Reference) (OtherBodyIndex :type Integer))
  (Class|StageEntityComponent|SetEntityState (Variables|Default|GetEntityComponent) 2 false))

(event Custom|GoToTop
  (Development|PrintString "Go Top")
  (bind _alpha (Timeline|ElevatorTimeline PlayFromStart)
    (:Update
      (Rendering|Debug|DrawDebugSphere (Math|Vector|Lerp(Vector) (Variables|Location|GetBottomLocation) (Variables|Location|GetTopLocation) _alpha) 1e+02 12 "(R=0.990167,G=1.000000,B=0.164100,A=1.000000)" 2.0 3.0)
      (Transformation|SetActorLocation (Math|Vector|Lerp(Vector) (Variables|Location|GetBottomLocation) (Variables|Location|GetTopLocation) _alpha) false false))))

(event Custom|GoToBottom
  (Development|PrintString "Go Bottom")
  (bind _alpha (Timeline|ElevatorTimeline Reverse)
    (:Update
      (Rendering|Debug|DrawDebugSphere (Math|Vector|Lerp(Vector) (Variables|Location|GetBottomLocation) (Variables|Location|GetTopLocation) _alpha) 1e+02 12 "(R=0.990167,G=1.000000,B=0.164100,A=1.000000)" 2.0 3.0)
      (Transformation|SetActorLocation (Math|Vector|Lerp(Vector) (Variables|Location|GetBottomLocation) (Variables|Location|GetTopLocation) _alpha) false false))))

(event Custom|ResetLocation
  (Development|PrintString "Reset Location")
  (Transformation|SetActorLocation (Variables|Location|GetBottomLocation) false false))

(event EventBeginPlay
  (|CallParentFunction)
  (Utilities|FlowControl|Delay 0.2)
  (bind _output_get (Variables|Location|SetBottomLocation (Transformation|GetActorLocation)))
  (Variables|Location|SetTopLocation (+ _output_get "0.000000,0.000000,500.000000"))
  (Rendering|Debug|DrawDebugSphere _output_get 1e+02 12 "(R=0.837373,G=1.000000,B=0.192322,A=1.000000)" 2.0 1.0))

(event Collision|EventActorBeginOverlap
  (params (OtherActor :type Actor%20Object%20Reference))
  (|CallParentFunction OtherActor) ; This node is disabled and will not be called.\nDrag off pins to build functionality.
)

(event EventTick
  (params (DeltaSeconds :type Float%20%28single-precision%29))
  (|CallParentFunction DeltaSeconds) ; This node is disabled and will not be called.\nDrag off pins to build functionality.
)

(fn ConstructionScript
  (|CallParentFunction))